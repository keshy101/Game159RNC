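; BP_Menu3D is a main-menu actor with a 3D widget that pans the camera between linked menu actors.
; On BeginPlay it binds the widget's transition event and disables its own collision.
; The event's index selects a LinkedMenu entry, whose collision is toggled off then on before an eased view-target blend makes it the player's view.
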(event Custom|TransitionTo
  (params (NewMenu :type BP%20Menu%203D%20Object%20Reference))
  ;[1 1 1] Camera Pan
  (Collision|SetActorEnableCollision NewMenu false)
  (Collision|SetActorEnableCollision NewMenu true)
  (Game|Player|SetViewTargetwithBlend (Game|GetPlayerController 0) NewMenu 3.0 "VTBlend_EaseInOut" 3.0 false))

(event Custom|OnTransitionBetweenMenu
  (params (MenuIndex :type Integer))
  ;[1 1 1] Transition from the menus
  (if (Utilities|Array|IsValidIndex (Variables|Default|GetLinkedMenu) MenuIndex)
    (CallFunction|Transitionto (Utilities|Array|Get(acopy) (Variables|Default|GetLinkedMenu) MenuIndex))))

(event EventBeginPlay
  ;[1 1 1] Transition from the menus
  (bind _asmenu_3dwidget (Utilities|Casting|CastToMenu3DWidget (UserInterface|GetUserWidgetObject (Variables|Default|GetWidget))))
  (EventDispatchers|AssignTransitiontoLinkedMenu _asmenu_3dwidget (delegate Custom|OnTransitionBetweenMenu))
  (Collision|SetActorEnableCollision false))

(fn ConstructionScript)