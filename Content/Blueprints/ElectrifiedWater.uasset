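; ElectrifiedWater is a water hazard that counts as electrified until the player fixes the electrical box.
; Every tick it finds the FirstPersonCharacter and stores the inverse of its ElecBoxFixed flag.
; A Delay on Tick spawns sparks at SparksSpawn roughly every two seconds while the hazard is live.
; DeathCollision overlaps only print a death or cold-water message, without checking the overlapping actor.
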(event OnComponentBeginOverlap(DeathCollision)
  (params (OverlappedComponent :type Primitive%20Component%20Object%20Reference) (OtherActor :type Actor%20Object%20Reference) (OtherComp :type Primitive%20Component%20Object%20Reference) (OtherBodyIndex :type Integer) (bFromSweep :type Boolean) (SweepResult :type Hit%20Result%20Structure%20%28by%20ref%29))
  (if (Variables|Default|GetElecBoxFixedInvert)
    (Development|PrintString "You Died!")
    (else
      (Development|PrintString "The water is murky and cold."))))

(event EventTick
  (params (DeltaSeconds :type Float%20%28single-precision%29))
  (Utilities|FlowControl|Sequence
    (:then_0
      (bind _outactors (Actor|GetAllActorsOfClass "/Game/Blueprints/FirstPersonCharacter.FirstPersonCharacter_C"))
      (if (Variables|/Game/Blueprints/FirstPersonCharacter.FirstPersonCharacter_C|GetElecBoxFixed (Utilities|Array|Get(acopy) _outactors))
        (Variables|Default|SetElecBoxFixedInvert false)
        (else
          (Variables|Default|SetElecBoxFixedInvert true))))
    (:then_1
      (Utilities|FlowControl|Delay 2.0)
      (if (Variables|Default|GetElecBoxFixedInvert)
        (Effects|SpawnEmitterAttached "/Game/Particles/SparksFinite.SparksFinite" (Variables|Default|GetSparksSpawn) "None")))))

(fn ConstructionScript)