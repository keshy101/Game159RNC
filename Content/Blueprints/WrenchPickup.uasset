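; WrenchPickup is a collectible wrench that the first-person character picks up by walking into it.
; Each tick it spins the static mesh around yaw at a Rotation speed scaled by delta time.
; When its collision component overlaps a FirstPersonCharacter, it sets that character's HasWrench flag, prints a message, plays a pickup sound and destroys itself.
; Other overlapping actors only trigger a debug print about the failed cast.
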(event OnComponentBeginOverlap(Collision)
  (params (OverlappedComponent :type Primitive%20Component%20Object%20Reference) (OtherActor :type Actor%20Object%20Reference) (OtherComp :type Primitive%20Component%20Object%20Reference) (OtherBodyIndex :type Integer) (bFromSweep :type Boolean) (SweepResult :type Hit%20Result%20Structure%20%28by%20ref%29))
  (bind _asfirst_person_character (Utilities|Casting|CastToFirstPersonCharacter OtherActor)
    (:then
      (Variables|/Game/Blueprints/FirstPersonCharacter.FirstPersonCharacter_C|SetHasWrench _asfirst_person_character true)
      (Development|PrintString "Picked up a wrench")
      (Audio|PlaySoundatLocation "/Game/Audio/pickup-sf.pickup-sf" (Transformation|GetActorLocation) "0, 0, 0" 1.0 1.0 0.0 0 0 0)
      (Actor|DestroyActor))
    (:CastFailed
      (Development|PrintString "cast failed in WrenchPickup"))))

(event EventTick
  (params (DeltaSeconds :type Float%20%28single-precision%29))
  (Transformation|AddWorldRotation (Variables|Default|GetStaticMesh) (Math|Rotator|MakeRotator 0.0 0.0 (* DeltaSeconds (Variables|Default|GetRotation))) false false))

(fn ConstructionScript)