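; ElectricalBox is an interactable broken electrical box that the player repairs with a wrench.
; When the FirstPersonCharacter overlaps its collision box, it checks HasWrench and prints a hint if the wrench is missing.
; With the wrench, it sets ElecBoxFixed on the character, destroys the trigger so the repair runs once, and plays a tightening sound and sparks effect.
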(event OnComponentBeginOverlap(BoxCollision)
  (params (OverlappedComponent :type Primitive%20Component%20Object%20Reference) (OtherActor :type Actor%20Object%20Reference) (OtherComp :type Primitive%20Component%20Object%20Reference) (OtherBodyIndex :type Integer) (bFromSweep :type Boolean) (SweepResult :type Hit%20Result%20Structure%20%28by%20ref%29))
  (bind _asfirst_person_character (Utilities|Casting|CastToFirstPersonCharacter OtherActor)
    (:then
      (if (Variables|/Game/Blueprints/FirstPersonCharacter.FirstPersonCharacter_C|GetHasWrench _asfirst_person_character)
        (bind _asfirst_person_character_2 (Utilities|Casting|CastToFirstPersonCharacter OtherActor)
          (:then
            (Variables|/Game/Blueprints/FirstPersonCharacter.FirstPersonCharacter_C|SetElecBoxFixed _asfirst_person_character_2 true)
            (Development|PrintString "There we go! Looks like it works now.")
            (Components|DestroyComponent (Variables|Default|GetBoxCollision))
            (Audio|PlaySoundatLocation "/Game/Audio/bolt-tightening-sf.bolt-tightening-sf" (Transformation|GetActorLocation) "0, 0, 0" 1.0 1.0 0.0 0 0 0)
            (Effects|SpawnEmitterAttached "/Game/Particles/SparksFinite.SparksFinite" (Variables|Default|GetParticleSpawn) "None" "0,0.000000, 0"))
          (:CastFailed
            (Development|PrintString "Cast failed in ElectricalBox")))
        (else
          (Development|PrintString "Looks like it short-circuited... Maybe I could fix it?"))))
    (:CastFailed
      (Development|PrintString "Cast failed in ElectricalBox"))))

(fn ConstructionScript)