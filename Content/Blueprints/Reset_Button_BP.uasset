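; Reset_Button_BP is a clickable actor named as a reset button, though it contains no reset logic.
; On click it enables input from player 0, updates CheckId with a modulo 1 increment that always yields zero, and calls SetMaterialByName on its static mesh.
; That call names slot None and supplies no material, while the Material1 and Material2 variables are unused, suggesting an unfinished material toggle.
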(event MouseInput|EventActorOnClicked
  (params (ButtonPressed :type Key%20Structure :default "None"))
  (Input|EnableInput (Game|GetPlayerController 0))
  (Variables|Default|SetCheck%20id (Math|Integer|%(Integer) (+ (Variables|Default|GetCheck%20id) 1) 1))
  (Rendering|Material|SetMaterialbyName (Variables|Debug|GetStaticMeshComponent) "None" 0))

(fn ConstructionScript
  (|CallParentFunction))